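; HUD Blueprint that draws a custom mouse cursor on screen with DrawMaterial.
; On each DrawHUD, it takes the mouse's viewport position and adds half the difference between the HUD size and viewport size.
; It then offsets by half the literal cursor dimensions, though the drawn height is also halved.
; The draw call shows no material assigned, and the other events are empty.
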(event EventBeginPlay)

(event Collision|EventActorBeginOverlap
  (params (OtherActor :type Actor%20Object%20Reference)))

(event EventTick
  (params (DeltaSeconds :type Float%20%28single-precision%29)))

(event EventDrawHUD
  (params (SizeX :type Integer) (SizeY :type Integer))
  (bind _returnvalue (Math|Float|MakeLiteralFloat 39.0))
  (bind _returnvalue_2 (Math|Float|MakeLiteralFloat 32.0))
  (bind _returnvalue_3 (Viewport|GetViewportSize))
  (bind (_x _y) (Math|Vector2D|BreakVector2D _returnvalue_3))
  (bind _returnvalue_4 (/ _returnvalue 2.0))
  (Canvas|DrawMaterial 0 (- (+ (/ (Math|Conversions|ToFloat(Integer) (- SizeX (Math|Float|Truncate _x))) 2.0) (.X (Math|Vector2D|BreakVector2D (stale _returnvalue)))) (/ _returnvalue_2 2.0)) (- (+ (.Y (Math|Vector2D|BreakVector2D (stale _returnvalue))) (/ (Math|Conversions|ToFloat(Integer) (- SizeY (Math|Float|Truncate _y))) 2.0)) _returnvalue_4) _returnvalue_2 _returnvalue_4 0.0 0.0 1.0 1.0))

(fn ConstructionScript)