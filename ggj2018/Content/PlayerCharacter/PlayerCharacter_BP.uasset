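; Player character Blueprint that can carry a flashlight, be used by other actors and be slowed down.
; Being used triggers SlowCharacter, as does a capsule hit with an AI character, with a smaller argument.
; Colliding with another player while holding the flashlight spawns a Flashlight_BP below and away from that player, then hides the cone and spotlight.
; CanUse simply returns the CanIBeUsed flag.
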(event `self.ReceiveBeginPlay`)

(event `/Game/AI_Playground/AI_Character/AI_Usable_Interface.Used`
  (params (UsingActor :type "Actor Object Reference") (Value :type Integer))
  (`self.SlowCharacter` "4.0f"))

(event `ChangeFlashlight`
  (bind _hasflashlight (`self.HasFlashlight`))
  (`SceneComponent.SetVisibility` (`self.Cone`) _hasflashlight true)
  (`SceneComponent.SetVisibility` (`self.SpotLight`) _hasflashlight true))

(event `self.CapsuleComponent.OnComponentHit`
  (params (HitComponent :type "PrimitiveComponent Object Reference") (OtherActor :type "Actor Object Reference") (OtherComp :type "PrimitiveComponent Object Reference") (NormalImpulse :type "Vector Structure") (Hit :type "HitResult Structure (by ref)"))
  (bind _returnvalue (`self.K2_GetActorLocation`))
  (if (`KismetMathLibrary.ClassIsChildOf` (`GameplayStatics.GetObjectClass` OtherActor) "/Script/ggj2018.AICharacter")
    (`self.SlowCharacter` 2.0)
    (elif (`KismetMathLibrary.ClassIsChildOf` (`GameplayStatics.GetObjectClass` OtherActor) "/Script/ggj2018.PlayerCharacter")
      (if (`self.HasFlashlight`)
        (`|SpawnActorFromClass` "/Game/Flashlight/Flashlight_BP.Flashlight_BP_C" (`KismetMathLibrary.MakeTransform` (+ _returnvalue (`KismetMathLibrary.MakeVector` (* 5.0 (- (.x _returnvalue) (.x (`self.K2_GetActorLocation` OtherActor)))) (* 5.0 (- (.y _returnvalue) (.y (`self.K2_GetActorLocation` OtherActor)))) -50.0))) "Undefined" "OverrideRootScale" null null)
        (`KismetSystemLibrary.PrintString` "Made a flashlight")
        (set `self.HasFlashlight` false)
        (`self.ChangeFlashlight`)))))

(fn `CanUse`
  (params (UsingActor :type "Actor Object Reference"))
  (returns (IsUsable :type Boolean))
  (return (`self.CanIBeUsed`)))

(fn `UserConstructionScript`)