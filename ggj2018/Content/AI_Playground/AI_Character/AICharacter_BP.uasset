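; AI character Blueprint with a ghost animation setup that can attack and take damage through use-style events.
; UseObject calls DoAttack on the mesh's GhostAnimBlueprint, using a DoOnce reset after a short delay to throttle repeat attacks.
; Used subtracts the incoming value from Health, with no death handling here.
; CanUse always returns false, and BeginPlay and the construction script are empty.
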(event `/Game/AI_Playground/AI_Character/AI_Usable_Interface.UseObject`
  (params (UsedObject :type "Actor Object Reference"))
  (`/Engine/EditorBlueprintResources/StandardMacros.DoOnce` false :!label _label
    (:`Completed`
      (bind _asghost_anim_blueprint (cast `/Game/Ghosts/GhostAnimBlueprint` (`SkeletalMeshComponent.GetAnimInstance` (`self.Mesh`))))
      (`/Game/Ghosts/GhostAnimBlueprint.DoAttack` _asghost_anim_blueprint)
      (`KismetSystemLibrary.Delay` 0.2)
      (goto _label :!via `Reset`))))

(event `/Game/AI_Playground/AI_Character/AI_Usable_Interface.Used`
  (params (UsingActor :type "Actor Object Reference") (Value :type Integer))
  (set `self.Health` (- (`self.Health`) Value)))

(event `self.ReceiveBeginPlay`)

(fn `CanUse`
  (params (UsingActor :type "Actor Object Reference"))
  (returns (IsUsable :type Boolean))
  (return false))

(fn `UserConstructionScript`)