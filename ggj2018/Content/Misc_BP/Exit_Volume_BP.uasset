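; Exit volume that moves the game to the next map when a flashlight-carrying player stays inside its box.
; Box overlap starts a timer of configurable length, calling the function named by NextLevelFunc, and leaving with the flashlight clears it.
; The NextLevel function opens the map set in NextMap.
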(event `self.Box.OnComponentBeginOverlap`
  (params (OverlappedComponent :type "PrimitiveComponent Object Reference") (OtherActor :type "Actor Object Reference") (OtherComp :type "PrimitiveComponent Object Reference") (OtherBodyIndex :type Integer) (bFromSweep :type Boolean) (SweepResult :type "HitResult Structure (by ref)"))
  (if (`KismetMathLibrary.ClassIsChildOf` (`GameplayStatics.GetObjectClass` OtherActor) "/Script/ggj2018.PlayerCharacter")
    (bind _asplayer_character_bp (cast `/Game/PlayerCharacter/PlayerCharacter_BP` OtherActor))
    (if (`PlayerCharacter.HasFlashlight` _asplayer_character_bp)
      (bind _returnvalue (`KismetSystemLibrary.K2_SetTimer` null (`self.NextLevelFunc`) (`self.ExitTimerLength`))))))

(event `self.Box.OnComponentEndOverlap`
  (params (OverlappedComponent :type "PrimitiveComponent Object Reference") (OtherActor :type "Actor Object Reference") (OtherComp :type "PrimitiveComponent Object Reference") (OtherBodyIndex :type Integer))
  (if (`KismetMathLibrary.ClassIsChildOf` (`GameplayStatics.GetObjectClass` OtherActor) "/Script/ggj2018.PlayerCharacter")
    (bind _asplayer_character_bp (cast `/Game/PlayerCharacter/PlayerCharacter_BP` OtherActor))
    (if (`PlayerCharacter.HasFlashlight` _asplayer_character_bp)
      (`KismetSystemLibrary.K2_ClearAndInvalidateTimerHandle` (stale `self.Box.OnComponentBeginOverlap` _returnvalue)))))

(fn `NextLevel`
  (`GameplayStatics.OpenLevel` (`self.NextMap`)))

(fn `UserConstructionScript`)